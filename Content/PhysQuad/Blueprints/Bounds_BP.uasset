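; Bounds_BP is an out-of-bounds trigger volume for the automated drones.
; When an actor begins overlapping the OutOfBound component, it tries casting it to four drone classes in sequence, Automate_Drone through Automate_Drone_4.
; The first successful cast calls that drone's OutBound function, and failures of the first three casts print a debug message before falling through.
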(event OnComponentBeginOverlap(OutOfBound)
  (params (OverlappedComponent :type Primitive%20Component%20Object%20Reference) (OtherActor :type Actor%20Object%20Reference) (OtherComp :type Primitive%20Component%20Object%20Reference) (OtherBodyIndex :type Integer) (bFromSweep :type Boolean) (SweepResult :type Hit%20Result%20Structure%20%28by%20ref%29))
  (bind _asautomate_drone (Utilities|Casting|CastToAutomate_Drone OtherActor)
    (:then
      (Default|OutBound _asautomate_drone))
    (:CastFailed
      (Development|PrintString "Cast Failed")
      (bind _asautomate_drone_2 (Utilities|Casting|CastToAutomate_Drone_2 OtherActor)
        (:then
          (Default|OutBound _asautomate_drone_2))
        (:CastFailed
          (Development|PrintString "Cast Failed")
          (bind _asautomate_drone_3 (Utilities|Casting|CastToAutomate_Drone_3 OtherActor)
            (:then
              (Default|OutBound _asautomate_drone_3))
            (:CastFailed
              (Development|PrintString "Cast Failed")
              (bind _asautomate_drone_4 (Utilities|Casting|CastToAutomate_Drone_4 OtherActor))
              (Default|OutBound _asautomate_drone_4))))))))

(event EventBeginPlay)

(event Collision|EventActorBeginOverlap
  (params (OtherActor :type Actor%20Object%20Reference)))

(event EventTick
  (params (DeltaSeconds :type Float%20%28single-precision%29)))

(fn ConstructionScript)